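; BP_Planet is a planet actor that orbits a center point while spinning on its own axis.
; The construction script scales the mesh from Radius and positions the actor from SunDistance and Radius.
; BeginPlay moves the actor's origin to Center, restores the axis root to the starting spot, and randomizes orbital yaw.
; Tick yaws actor and mesh at speeds inversely proportional to OrbitalPeriod and DayLength, so rotating the actor produces the orbit.
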(event EventBeginPlay
  (Variables|Default|SetInitial%20Planet%20Location (Transformation|GetActorTransform))
  (Transformation|SetActorLocationAndRotation (Variables|Default|GetCenter) "0, 0, 0")
  (Transformation|SetWorldLocationAndRotation (Variables|Default|GetPlanet%20Axis%20Root) (.location (Variables|Default|GetInitial%20Planet%20Location)) (.rotation (Variables|Default|GetInitial%20Planet%20Location)) false false)
  (Transformation|SetActorRotation (Math|Rotator|MakeRotator 0.0 0.0 (Math|Random|RandomFloatinRange 0.0 3.6e+02))))

(event Collision|EventActorBeginOverlap
  (params (OtherActor :type Actor%20Object%20Reference)))

(event EventTick
  (params (DeltaSeconds :type Float%20%28single-precision%29))
  (bind _sm_planet (Variables|Default|GetSM_Planet))
  (Transformation|SetActorRotation (Math|Rotator|MakeRotator 0.0 0.0 (+ (.yaw (Transformation|GetActorRotation)) (* DeltaSeconds 2e+01 (/ 88.0 (Variables|Default|GetOrbital%20Period))))))
  (Transformation|SetRelativeRotation _sm_planet (Math|Rotator|MakeRotator 0.0 0.0 (+ (.yaw (Variables|/Script/Engine.SceneComponent|GetRelativeRotation _sm_planet)) (* (Utilities|Time|GetWorldDeltaSeconds) 0.5 (/ 58.0 (Variables|Default|GetDay%20Length))))) false false))

(fn ConstructionScript
  (Transformation|SetWorldScale3D (Variables|Default|GetSM_Planet) (Math|Conversions|ToVector(Float) (/ (Variables|Default|GetRadius) 85.0)))
  (Transformation|SetActorLocation (Math|Vector|MakeVector (Variables|Default|GetSun%20Distance) (- 0.0 (/ (Variables|Default|GetRadius) 2.0)) 0.0) false false))